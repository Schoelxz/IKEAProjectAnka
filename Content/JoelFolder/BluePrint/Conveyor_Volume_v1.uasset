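; Conveyor volume that carries every overlapping actor along its forward direction at a set Speed.
; Each Tick it offsets those actors by the forward vector scaled by Speed and delta time, without sweep, so the move ignores blocking collision.
; The construction script counter-scales the Arrow component so it keeps a constant size when the volume is resized.
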(event `self.ReceiveTick`
  (params (DeltaSeconds :type "Float (single-precision)"))
  (for _array_element (`self.GetOverlappingActors` null)
    (`self.K2_AddActorWorldOffset` _array_element (* (`KismetMathLibrary.GetForwardVector` (`self.K2_GetActorRotation`)) (* DeltaSeconds (`self.Speed`))) false false)))

(fn `UserConstructionScript`
  (`SceneComponent.SetRelativeScale3D` (`self.Arrow`) (/ (1.0 1.0 1.0) (`self.GetActorScale3D`))))