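; AI pawn that spins constantly on yaw and moves toward the player's FirstPersonCharacter once PawnSensing sees it.
; A sighting sets IfSeePlayer and starts AIMoveTo, with a DoOnce playing a sound call at the pawn's location, though no sound asset is set.
; Tick rotates it regardless of sighting: IfSeePlayer is never read, and the loop that would clear it never runs.
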(event `self.PawnSensing.OnSeePawn`
  (params (Pawn :type "Pawn Object Reference"))
  (while false
    (set `self.ifSeePlayer` false))
  (set `self.ifSeePlayer` true)
  ;[1 1 1] Self moves to Player
  (bind _asfirst_person_character (cast `/Game/FirstPersonBP/Blueprints/FirstPersonCharacter` Pawn))
  (`|AIMoveTo` self (0.0 0.0 0.0) _asfirst_person_character 100.0
    (:`then`
      (`/Engine/EditorBlueprintResources/StandardMacros.DoOnce` false
        (:`Completed`
          (`GameplayStatics.PlaySoundAtLocation` null (`self.K2_GetActorLocation`)))))))

(event `self.ReceiveTick`
  (params (DeltaSeconds :type "Float (single-precision)"))
  (if (not false)
    (`self.K2_AddActorWorldRotation` (* (`KismetMathLibrary.MakeRotator` 0.0 0.0 100.0) DeltaSeconds))))

(fn `UserConstructionScript`)